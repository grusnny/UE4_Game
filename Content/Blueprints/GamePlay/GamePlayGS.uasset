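; GamePlayGS is the gameplay game state, handling match result, match exit and the player stats screen.
; ActualizarEstado stores the winner name and victory state, while Finalizarpartida has GameInfoInstance destroy the session and opens the MainMenu level.
; LaunchStats creates a StatsList widget, fills it from each GamePlayPS player state in PlayerArray and adds it to the viewport.
; CloseStats removes that widget.
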(event `ActualizarEstado`
  (params (Nombre :type Text) (Estado :type Boolean))
  (set `self.NombreGanador` Nombre)
  (set `self.Victoria?` Estado))

(event `Finalizar partida`
  (bind _asgame_info_instance (cast `/Game/Blueprints/AllLevels/GameInfoInstance` (`GameplayStatics.GetGameInstance`)))
  (`/Game/Blueprints/AllLevels/GameInfoInstance.DestroySessionCaller` _asgame_info_instance (`GameplayStatics.GetPlayerController` 0))
  (`GameplayStatics.OpenLevel` "MainMenu"))

(event `LaunchStats`
  (bind _returnvalue (`|CreateWidget` "/Game/UI/AllLevels/StatsList.StatsList_C"))
  (bind _output_get (set `self.RefPlayerStas` _returnvalue))
  (`/Game/UI/AllLevels/StatsList.ClearPlayerList` _output_get)
  (for _array_element (`self.PlayerArray`)
    (bind _asgame_play_ps (cast `/Game/Blueprints/GamePlay/GamePlayPS` _array_element))
    (`/Game/UI/AllLevels/StatsList.UpdatePlayerWindow` _returnvalue (`/Game/Blueprints/GamePlay/GamePlayPS.PlayerInfo` _asgame_play_ps) _asgame_play_ps null))
  (`UserWidget.AddToViewport` _returnvalue 0))

(event `CloseStats`
  (bind _refplayerstas (`self.RefPlayerStas`))
  (`/Engine/EditorBlueprintResources/StandardMacros.IsValid` _refplayerstas
    (:`Is Valid`
      (`Widget.RemoveFromParent` _refplayerstas))))

(fn `UserConstructionScript`)